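; Base interactable actor for the digital twin editor, tracking selection focus and customisation state.
; Selection, regular and post-creation customisation interface events set state flags, fire Call hooks and swap every static mesh to debug materials.
; A primary click during focused customisation tells the player pawn to confirm and end it; otherwise it only logs.
; Cancelling post-creation customisation destroys the actor, while cancelling regular customisation keeps it.
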(event `/Game/BPs/Interfaces/ExtendedClickingInterface.PrimaryClick`
  (params (Clicker :type "Actor Object Reference") (ClickHit :type "HitResult Structure"))
  (`self.RecievedPrimaryClick`)
  (if (and (`self.IsBeeingCustomised`) (`self.IsSelectionFocus`))
    ;[1 1 1] If clicked on during customisation, confirm and end customisation.
    (`/Game/BPs/Utilitys/ErrorAndWarningSignals.PrintDebugLog` (`KismetStringLibrary.Concat_StrStr` "I was clicked on by " (`KismetSystemLibrary.GetDisplayName` Clicker) " during my customisation!") self)
    (message `/Game/BPs/Interfaces/CustomisationInterface.NotifyPawnOfEndOfCustomisation` (`GameplayStatics.GetPlayerPawn` 0) "NewEnumerator0")
    (else
      (bind _asbp_digital_twin_editor_pawn (cast `/Game/BPs/Core/BP_DigitalTwin_EditorPawn` (`GameplayStatics.GetPlayerPawn` 0)))
      (if (== (`/Game/BPs/Core/BP_DigitalTwin_EditorPawn.GetSelectedReferences` _asbp_digital_twin_editor_pawn) self)
        (`/Game/BPs/Utilitys/ErrorAndWarningSignals.PrintDebugLog` "I was left clicked, ready to be moved!" self)
        (else
          (`/Game/BPs/Utilitys/ErrorAndWarningSignals.PrintWarning` "I was left-clicked during some other objects customisation. Ignoring Click for now..." self))))))

(event `/Game/BPs/Interfaces/SelectionInterface.RegisterSelection`
  ;[1 1 1] Selection Interface
  (set `self.IsSelectionFocus` true)
  (`self.BeginFocus`)
  (`/Game/BPs/Utilitys/ErrorAndWarningSignals.PrintDebugLog` "I have been selected!" self)
  ;;[1 1 1] Debug Paint
  (for _array_element (`self.K2_GetComponentsByClass` "/Script/Engine.StaticMeshComponent")
    (`PrimitiveComponent.SetMaterial` _array_element 0 "/Game/Materials/mat_Debug_blue.mat_Debug_blue")))

(event `/Game/BPs/Interfaces/SelectionInterface.UnRegisterSelection`
  ;[1 1 1] Selection Interface
  (set `self.IsSelectionFocus` false)
  (`self.EndFocus`)
  (`/Game/BPs/Utilitys/ErrorAndWarningSignals.PrintDebugLog` "I have been unselected!" self)
  ;;[1 1 1] Debug Paint
  (for _array_element (`self.K2_GetComponentsByClass` "/Script/Engine.StaticMeshComponent")
    (`PrimitiveComponent.SetMaterial` _array_element 0 "/Engine/EngineMaterials/WorldGridMaterial.WorldGridMaterial")))

(event `/Game/BPs/Interfaces/CustomisationInterface.InitRegularCustomisation`
  ;[1 1 1] Regular Customisation Interface
  (set `self.IsBeeingCustomised` true)
  (`self.BeginCustomisation`)
  (`/Game/BPs/Utilitys/ErrorAndWarningSignals.PrintDebugLog` "I am beeing customised!" self)
  (for _array_element (`self.K2_GetComponentsByClass` "/Script/Engine.StaticMeshComponent")
    (`PrimitiveComponent.SetMaterial` _array_element 0 "/Game/Materials/mat_Debug_green.mat_Debug_green")))

(event `/Game/BPs/Interfaces/CustomisationInterface.EndRegularCustomisation`
  (params (EndType :type "/Game/BPs/Customisation/Enums/SubModeExitType Enum" :default "NewEnumerator0"))
  ;[1 1 1] Regular Customisation Interface
  (set `self.IsBeeingCustomised` false)
  (`self.EndCustomisation`)
  (switch `/Game/BPs/Customisation/Enums/SubModeExitType` EndType
    (:`NewEnumerator0`
      (`/Game/BPs/Utilitys/ErrorAndWarningSignals.PrintDebugLog` "My customisation was completed!" self))
    (:`NewEnumerator1`
      (`/Game/BPs/Utilitys/ErrorAndWarningSignals.PrintDebugLog` "My customisation as caceled!" self)))
  (for _array_element (`self.K2_GetComponentsByClass` "/Script/Engine.StaticMeshComponent")
    (`PrimitiveComponent.SetMaterial` _array_element 0 "/Game/Materials/mat_Debug_blue.mat_Debug_blue")))

(event `/Game/BPs/Interfaces/CustomisationInterface.InitPostCreationCustomisation`
  ;[1 1 1] Spawn Customisation Interface
  ;;[1 1 1] Actor is just spawning in, use this event to customise the Actor on Spawn!
  (set `self.IsBeeingCustomised` true)
  (`self.BeginCustomisation`)
  (`/Game/BPs/Utilitys/ErrorAndWarningSignals.PrintDebugLog` "I am beeing customised after beeing spawned!" self)
  (for _array_element (`self.K2_GetComponentsByClass` "/Script/Engine.StaticMeshComponent")
    (`PrimitiveComponent.SetMaterial` _array_element 0 "/Game/Materials/mat_Debug_green.mat_Debug_green")))

(event `/Game/BPs/Interfaces/CustomisationInterface.EndPostCreationCustomisation`
  (params (EndType :type "/Game/BPs/Customisation/Enums/SubModeExitType Enum" :default "NewEnumerator0"))
  ;[1 1 1] Spawn Customisation Interface
  ;;[1 1 1] Actor is just spawning in, use this event to customise the Actor on Spawn!
  (set `self.IsBeeingCustomised` false)
  (`self.EndCustomisation`)
  (switch `/Game/BPs/Customisation/Enums/SubModeExitType` EndType
    (:`NewEnumerator0`
      (`/Game/BPs/Utilitys/ErrorAndWarningSignals.PrintDebugLog` "My initial customisation was completed!" self)
      (for _array_element (`self.K2_GetComponentsByClass` "/Script/Engine.StaticMeshComponent")
        (`PrimitiveComponent.SetMaterial` _array_element 0 "/Game/Materials/mat_Debug_blue.mat_Debug_blue")))
    (:`NewEnumerator1`
      (`/Game/BPs/Utilitys/ErrorAndWarningSignals.PrintDebugLog` "My initial customisation was canceled! Goodbye cruel world!" self)
      (`self.K2_DestroyActor`))))

(fn `CreationCustomisation`)

(fn `UpdateSelectionFocus`
  (params (`New IsSelectionFocus` :type Boolean))
  (set `self.IsSelectionFocus` `New IsSelectionFocus`))

(fn `UserConstructionScript`)