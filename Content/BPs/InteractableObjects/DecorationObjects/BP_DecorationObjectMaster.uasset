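; Base Blueprint for decoration objects that can be dragged across a grid with the mouse in the digital twin editor.
; A primary click enables Tick when the object has selection focus and is not being customised, and releasing disables it.
; Each Tick snaps the cursor's visibility-trace XY to the grid at the current height, passes it to the EditorUI slider position and moves the actor there.
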(event `/Game/BPs/Interfaces/ExtendedClickingInterface.PrimaryClick`
  (params (Clicker :type "Actor Object Reference") (ClickHit :type "HitResult Structure"))
  ;[1 1 1] Check if Object was clicked
  (`parent.PrimaryClick` Clicker ClickHit)
  (if (and (`self.IsSelectionFocus`) (not (`self.IsBeeingCustomised`)))
    (`self.SetActorTickEnabled` true)))

(event `self.ReceiveTick`
  (params (DeltaSeconds :type "Float (single-precision)"))
  (bind _gridalignedposition (`/Game/BPs/Utilitys/GridSystem.SnapLocationToGrid` (`KismetMathLibrary.MakeVector` (.x (`.Location` (`GameplayStatics.BreakHitResult` (`PlayerController.GetHitResultUnderCursorByChannel` (`GameplayStatics.GetPlayerController` 0) "TraceTypeQuery1" true)))) (.y (`.Location` (`GameplayStatics.BreakHitResult` (`PlayerController.GetHitResultUnderCursorByChannel` (`GameplayStatics.GetPlayerController` 0) "TraceTypeQuery1" true)))) (.z (`self.K2_GetActorLocation`)))))
  ;[1 1 1] Engage Object movement with mouse cursor
  (bind _asbp_digital_twin_editor_pawn (cast `/Game/BPs/Core/BP_DigitalTwin_EditorPawn` (`GameplayStatics.GetPlayerPawn` 0)))
  (bind _aseditor_ui (cast `/Game/UMG/EditorUI` (`/Game/BPs/Core/BP_DigitalTwin_EditorPawn.MainEditorUI` _asbp_digital_twin_editor_pawn)))
  (`/Game/UMG/EditorUI.Set Slider Position` _aseditor_ui _gridalignedposition)
  (`self.K2_SetActorLocation` _gridalignedposition))

(event `/Game/BPs/Interfaces/ExtendedClickingInterface.PrimaryUnClick`
  ;[1 1 1] Check if Object was clicked
  (`parent.PrimaryUnClick`)
  (if (`self.IsActorTickEnabled`)
    (`self.SetActorTickEnabled` false)))

(fn `UserConstructionScript`
  (`parent.UserConstructionScript`))