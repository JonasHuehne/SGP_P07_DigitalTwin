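; BP_DigitalTwin_GameInstance is a Game Instance that holds session settings and level handoff data for the digital twin app.
; Small update functions write location snap, rotation snap and ground trace values into the SessionSettings struct.
; StoreNewLevelInfo saves an Area and raises the HasHotLevelInfo flag, and ReturnNewLevelInfo clears that flag and returns the stored Area.
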(fn `GroundTrace_Update`
  (params (NewValue :type Boolean))
  (setmembers `/Game/BPs/Core/SettingsStruct` :`StructRef` (`self.SessionSettings`) :`GroundTrace` NewValue))

(fn `LocSnap_Update`
  (params (`New Value` :type Boolean))
  (setmembers `/Game/BPs/Core/SettingsStruct` :`StructRef` (`self.SessionSettings`) :`LocSnap` `New Value`))

(fn `ReturnNewLevelInfo`
  (returns (Area :type "Vector2D Structure"))
  (set `self.HasHotLevelInfo` false)
  (return (`self.Area`)))

(fn `RotSnap_Update`
  (params (NewValue :type Boolean))
  (setmembers `/Game/BPs/Core/SettingsStruct` :`StructRef` (`self.SessionSettings`) :`RotSnap` NewValue))

(fn `StoreNewLevelInfo`
  (params (Area :type "Vector2D Structure"))
  (set `self.HasHotLevelInfo` true)
  (set `self.Area` Area))