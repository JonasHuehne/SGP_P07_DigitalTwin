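; Player pawn for a digital-twin editor, switching between an orthographic top-down view and a first-person view, with axis movement, zoom and hold-to-rotate mouse look.
; Mouse clicks spawn, select and customise scene objects, tracking selection and customisation state and forwarding messages to those objects.
; It creates the EditorUI, updating it on selection and scene changes.
; Perspective switches ground-trace the first-person position and toggle SunSky shadows.
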(event `self.ReceiveTick`
  (params (DeltaSeconds :type "Float (single-precision)"))
  (bind (_returnvalue_x _returnvalue_y) (`KismetMathLibrary.BreakVector2D` (`WidgetLayoutLibrary.GetViewportSize`)))
  (bind (_prevmouse_x _prevmouse_y) (`KismetMathLibrary.BreakVector2D` (`self.PrevMouse`)))
  (bind _returnvalue (`KismetMathLibrary.FTrunc` _prevmouse_y))
  (bind _returnvalue_2 (`KismetMathLibrary.FTrunc` _prevmouse_x))
  (bind _returnvalue_3 (`KismetMathLibrary.FTrunc` (/ _returnvalue_x 2.0)))
  (bind _returnvalue_4 (`KismetMathLibrary.FTrunc` (/ _returnvalue_y 2.0)))
  ;[1 1 1] Update Mouse Delta
  (bind _asplayer_controller (cast `PlayerController` (`self.GetController`)))
  (if (not (`PlayerController.bShowMouseCursor` _asplayer_controller))
    (bind (_locationx _locationy) (`PlayerController.GetMousePosition` _asplayer_controller))
    (bind _returnvalue_5 (`KismetMathLibrary.MakeVector2D` _locationx _locationy))
    (bind _output_get (set `self.MouseDelta` (- _returnvalue_5 (`self.PrevMouse`))))
    (set `self.PrevMouse` _returnvalue_5)
    (bind (_x _y) (`KismetMathLibrary.BreakVector2D` _output_get))
    (if (== _x 0.0)
      (bind _returnvalue_6 (== _y 0.0))
      (if _returnvalue_6
        (`PlayerController.SetMouseLocation` _asplayer_controller _returnvalue_3 _returnvalue_4)
        (set `self.PrevMouse` (`KismetMathLibrary.MakeVector2D` (`KismetMathLibrary.Conv_IntToDouble` _returnvalue_3) (`KismetMathLibrary.Conv_IntToDouble` _returnvalue_4)))
        (else
          (`PlayerController.SetMouseLocation` _asplayer_controller _returnvalue_3 _returnvalue)
          (set `self.PrevMouse` (`KismetMathLibrary.MakeVector2D` (`KismetMathLibrary.Conv_IntToDouble` _returnvalue_3) (`KismetMathLibrary.Conv_IntToDouble` _returnvalue)))))
      (elif _returnvalue_6
        (`PlayerController.SetMouseLocation` _asplayer_controller _returnvalue_2 _returnvalue_4)
        (set `self.PrevMouse` (`KismetMathLibrary.MakeVector2D` (`KismetMathLibrary.Conv_IntToDouble` _returnvalue_2) (`KismetMathLibrary.Conv_IntToDouble` _returnvalue_4)))))))

(event `self.ReceiveBeginPlay`
  ;[1 1 1] Create Debug UI
  (bind _returnvalue (`|CreateWidget` "/Game/UMG/EditorUI.EditorUI_C"))
  (bind _output_get (set `self.MainEditorUI` _returnvalue))
  (`UserWidget.AddToViewport` _output_get 0))

(event `Key|H`
  (params (Key :type "Key Structure"))
  (:`Pressed`
    (bind _aseditor_ui (cast `/Game/UMG/EditorUI` (`self.MainEditorUI`)))
    (`/Game/UMG/EditorUI.toggleAllVisible` _aseditor_ui)))

(event `Key|One`
  (params (Key :type "Key Structure"))
  ;[0.9041 0 1] Debug
  (:`Pressed`
    (`self.SelectNewObject` null "/Game/BPs/InteractableObjects/ArchitecturalObjects/ExampleWall.ExampleWall_C")
    (`/Game/BPs/Utilitys/ErrorAndWarningSignals.PrintDebugLog` "Debug Selection Set to Wall!" self)))

(event `/Game/BPs/Interfaces/CustomisationInterface.NotifyPawnOfEndOfCustomisation`
  (params (ResultOfCustomisation :type "/Game/BPs/Customisation/Enums/SubModeExitType Enum" :default "NewEnumerator0"))
  ;[1 1 1] Object reports customisation completed!
  (`self.ExitCustomisation` ResultOfCustomisation)
  (bind _aseditor_ui (cast `/Game/UMG/EditorUI` (`self.MainEditorUI`)))
  (`/Game/UMG/EditorUI.RefreshSceneList` _aseditor_ui))

(event `InputAxis|AxisForward`
  (params (AxisValue :type "Float (single-precision)"))
  (bind _returnvalue (`GameplayStatics.GetWorldDeltaSeconds`))
  (bind _returnvalue_2 (!= AxisValue 0.0))
  (bind _movementspeed (`self.MovementSpeed`))
  ;[1 1 1] Basic Orthographic Movement
  ;;[1 1 1] If Input Exists
  (if _returnvalue_2
    ;;[1 1 1] Smooth Acceleration
    (bind _output_get (set `self.MovementSpeed` (`KismetMathLibrary.FInterpTo` _movementspeed (`self.SpeedMax`) _returnvalue (`self.Acceleration`))))
    ;;[1 1 1] Apply Actor Offset
    (`self.K2_AddActorLocalOffset` (`KismetMathLibrary.MakeVector` (* _output_get (`KismetMathLibrary.SignOfFloat` AxisValue) _returnvalue)))
    (else
      ;;[1 1 1] Slow down if no Input
      (if (`KismetMathLibrary.BooleanNOR` _returnvalue_2 (!= (stale `InputAxis|AxisRight` AxisValue) 0.0))
        (set `self.MovementSpeed` (`KismetMathLibrary.FInterpTo` _movementspeed 0.0 _returnvalue 2.0))))))

(event `InputAxis|AxisRight`
  (params (AxisValue :type "Float (single-precision)"))
  (bind _returnvalue (`GameplayStatics.GetWorldDeltaSeconds`))
  ;[1 1 1] Basic Orthographic Movement
  ;;[1 1 1] If Input Exists
  (if (!= AxisValue 0.0)
    ;;[1 1 1] Smooth Acceleration
    (bind _output_get (set `self.MovementSpeed` (`KismetMathLibrary.FInterpTo` (`self.MovementSpeed`) (`self.SpeedMax`) _returnvalue (`self.Acceleration`))))
    ;;[1 1 1] Apply Actor Offset
    (`self.K2_AddActorLocalOffset` (`KismetMathLibrary.MakeVector` 0.0 (* _output_get (`KismetMathLibrary.SignOfFloat` AxisValue) _returnvalue)))))

(event `InputAction|ActionLMB`
  (params (Key :type "Key Structure"))
  (bind _selectedactor (`self.SelectedActor`))
  (bind _hitresult (`PlayerController.GetHitResultUnderCursorForObjects` (`GameplayStatics.GetPlayerController` 0) (`|MakeArray` "ObjectTypeQuery1" "ObjectTypeQuery2" "ObjectTypeQuery7" :!type "EObjectTypeQuery Enum") true))
  (bind (_bblockinghit _binitialoverlap _time _distance _location _impactpoint _normal _impactnormal _physmat _hitactor) (`GameplayStatics.BreakHitResult` _hitresult))
  ;[1 1 1] Click-Based Interactions
  (:`Pressed`
    (`self.IsShowCursor`
      (:`True`
        ;;[1 1 1] If not customising current Object
        (if (or (`self.IsInSpawnCustomisation`) (`self.IsInRegularCustomisation`) (== _hitactor _selectedactor))
          (`/Game/BPs/Utilitys/ErrorAndWarningSignals.PrintDebugLog` "LeftClick during Customisation on customised Object." self)
          ;;[1 1 1] LeftClick onto Object beeing customised!
          (message `/Game/BPs/Interfaces/ExtendedClickingInterface.PrimaryClick` (`self.SelectedActor`) self (struct))
          (else
            ;;[1 1 1] Either spawn new Object if such an object is selected to be spawned or select existing object.
            (if (`self.IsInSpawnInMode`)
              (`self.SpawnNewObject` _hitresult)
              (else
                (`self.SelectNewObject` _hitactor))))))))
  (:`Released`
    (`self.PrimaryUnClickEvent`)
    (`/Engine/EditorBlueprintResources/StandardMacros.IsValid` _selectedactor
      (:`Is Valid`
        (message `/Game/BPs/Interfaces/ExtendedClickingInterface.PrimaryUnClick` _selectedactor)))))

(event `InputAction|ActionZoomOut`
  (params (Key :type "Key Structure"))
  (bind _topdowncamera (`self.TopDownCamera`))
  (bind _orthowidth (`CameraComponent.OrthoWidth` _topdowncamera))
  ;[1 1 1] Zoom by setting FOV for ortho. Camera
  (:`Pressed`
    (`CameraComponent.SetOrthoWidth` _topdowncamera (`KismetMathLibrary.FClamp` (+ (* _orthowidth 0.1) _orthowidth) 256.0 10240.0))))

(event `InputAction|ActionZoomIn`
  (params (Key :type "Key Structure"))
  (bind _topdowncamera (`self.TopDownCamera`))
  (bind _orthowidth (`CameraComponent.OrthoWidth` _topdowncamera))
  ;[1 1 1] Zoom by setting FOV for ortho. Camera
  (:`Pressed`
    (`CameraComponent.SetOrthoWidth` _topdowncamera (`KismetMathLibrary.FClamp` (+ (* _orthowidth -0.1) _orthowidth) 256.0 10240.0))))

(event `InputAction|ActionRMB`
  (params (Key :type "Key Structure"))
  (bind _selectedactor (`self.SelectedActor`))
  (bind (_bblockinghit _binitialoverlap _time _distance _location _impactpoint _normal _impactnormal _physmat _hitactor) (`GameplayStatics.BreakHitResult` (`PlayerController.GetHitResultUnderCursorForObjects` (`GameplayStatics.GetPlayerController` 0) (`|MakeArray` "ObjectTypeQuery1" "ObjectTypeQuery2" "ObjectTypeQuery7" :!type "EObjectTypeQuery Enum") true)))
  ;[1 1 1] Click-Based Interactions
  (:`Pressed`
    (`self.IsShowCursor`
      (:`True`
        ;;[1 1 1] If currently customising an object...
        (if (or (`self.IsInSpawnCustomisation`) (`self.IsInRegularCustomisation`))
          ;;[1 1 1] ... cancel the customisation
          (`self.ExitCustomisation` "NewEnumerator1")
          (else
            ;;[1 1 1] Otherwise, enter customisation if object was in focus, or set it to focus and enter customisation.
            (if (`self.HasValidClassSelection`)
              (`self.CancelPlacement`)
              (else
                (if (not (and (`self.HasValidActorSelection`) (== _hitactor (`self.SelectedActor`))))
                  (`self.SelectNewObject` _hitactor))
                (`self.EnterCustomisation` _hitactor "NewEnumerator1"))))))))
  (:`Released`
    (`self.SecondaryUnClickEvent`)
    (`/Engine/EditorBlueprintResources/StandardMacros.IsValid` _selectedactor
      (:`Is Valid`
        (message `/Game/BPs/Interfaces/ExtendedClickingInterface.SecondaryUnClick` _selectedactor)))))

(event `InputAction|SwitchPerspectives`
  (params (Key :type "Key Structure"))
  ;[1 1 1] Perpective Switch
  (:`Pressed`
    (set `self.IsFirstPerson` (not (`self.IsFirstPerson`)))
    (`self.UpdatePerspective`)))

(event `InputAction|ActionMMB`
  (params (Key :type "Key Structure"))
  (bind _selectedactor (`self.SelectedActor`))
  (bind _hitresult (`PlayerController.GetHitResultUnderCursorForObjects` (`GameplayStatics.GetPlayerController` 0) (`|MakeArray` "ObjectTypeQuery1" "ObjectTypeQuery2" "ObjectTypeQuery7" :!type "EObjectTypeQuery Enum") true))
  (bind (_bblockinghit _binitialoverlap _time _distance _location _impactpoint _normal _impactnormal _physmat _hitactor) (`GameplayStatics.BreakHitResult` _hitresult))
  ;[1 1 1] Click-Based Interactions
  (:`Pressed`
    (`self.IsShowCursor`
      (:`True`
        (if (and (`self.HasValidActorSelection`) (== _hitactor (`self.SelectedActor`)))
          (`self.UnSelectCurrentSelection`))
        (message `/Game/BPs/Interfaces/ExtendedClickingInterface.TertiaryClick` _hitactor self _hitresult))))
  (:`Released`
    (`self.TertiaryUnClickEvent`)
    (`/Engine/EditorBlueprintResources/StandardMacros.IsValid` _selectedactor
      (:`Is Valid`
        (message `/Game/BPs/Interfaces/ExtendedClickingInterface.TertiaryUnClick` _selectedactor)))))

(event `InputAxis|MouseY`
  (params (AxisValue :type "Float (single-precision)"))
  (bind (_mousedelta_x _mousedelta_y) (`KismetMathLibrary.BreakVector2D` (`self.MouseDelta`)))
  ;[1 1 1] CameraRotation
  (`/Engine/EditorBlueprintResources/StandardMacros.Gate` true :!label _label
    (:`Exit`
      (`self.K2_AddActorLocalRotation` (`KismetMathLibrary.MakeRotator` 0.0 (* _mousedelta_y 12.0 (`GameplayStatics.GetWorldDeltaSeconds`) -1.0))))))

(event `InputAxis|MouseX`
  (params (AxisValue :type "Float (single-precision)"))
  (bind (_mousedelta_x _mousedelta_y) (`KismetMathLibrary.BreakVector2D` (`self.MouseDelta`)))
  ;[1 1 1] CameraRotation
  (`/Engine/EditorBlueprintResources/StandardMacros.Gate` true :!label _label_2
    (:`Exit`
      (`self.K2_AddActorWorldRotation` (`KismetMathLibrary.MakeRotator` 0.0 0.0 (* _mousedelta_x 12.0 (`GameplayStatics.GetWorldDeltaSeconds`)))))))

(event `InputAction|Alternative`
  (params (Key :type "Key Structure"))
  (bind (_mouseresetloc_x _mouseresetloc_y) (`KismetMathLibrary.BreakVector2D` (`self.MouseResetLoc`)))
  ;[1 1 1] CameraRotation
  (:`Pressed`
    (`|ExecutionSequence`
      (:`then_0`
        (goto _label_2 :!via `Open`))
      (:`then_1`
        (goto _label :!via `Open`))
      (:`then_2`
        (bind _asplayer_controller (cast `PlayerController` (`self.GetController`)))
        (set `PlayerController.bShowMouseCursor` false _asplayer_controller)
        (bind (_locationx _locationy) (`PlayerController.GetMousePosition` _asplayer_controller))
        (bind _output_get (set `self.MouseResetLoc` (`KismetMathLibrary.MakeVector2D` _locationx _locationy)))
        (set `self.PrevMouse` _output_get)
        (`GameplayStatics.SetViewportMouseCaptureMode` "CapturePermanently_IncludingInitialMouseDown"))))
  (:`Released`
    (`|ExecutionSequence`
      (:`then_0`
        (goto _label_2 :!via `Close`))
      (:`then_1`
        (goto _label :!via `Close`))
      (:`then_2`
        (bind _asplayer_controller_2 (cast `PlayerController` (`self.GetController`)))
        (set `PlayerController.bShowMouseCursor` true _asplayer_controller_2)
        (`PlayerController.SetMouseLocation` _asplayer_controller_2 (`KismetMathLibrary.FTrunc` _mouseresetloc_x) (`KismetMathLibrary.FTrunc` _mouseresetloc_y))
        (`GameplayStatics.SetViewportMouseCaptureMode` "CapturePermanently_IncludingInitialMouseDown")))))

(fn `CancelPlacement`
  (`/Game/BPs/Utilitys/ErrorAndWarningSignals.PrintDebugLog` "Cancelling Placement of Object!" self)
  (`self.UnSelectCurrentSelection`))

(fn `EnterCustomisation`
  (params (`Object to customise` :type "Actor Object Reference") (`Type of Customisation` :type "/Game/BPs/Customisation/Enums/CustomisationTypes Enum" :default "NewEnumerator0"))
  (if (`KismetSystemLibrary.IsValid` `Object to customise`)
    (switch `/Game/BPs/Customisation/Enums/CustomisationTypes` `Type of Customisation`
      (:`NewEnumerator0`
        ;[1 1 1] Set local Values
        (set `self.IsInSpawnCustomisation` true)
        (set `self.IsInRegularCustomisation` false)
        (`/Game/BPs/Utilitys/ErrorAndWarningSignals.PrintDebugLog` "Entering PostCreationCustomisation!" self)
        (message `/Game/BPs/Interfaces/CustomisationInterface.InitPostCreationCustomisation` `Object to customise`))
      (:`NewEnumerator1`
        (set `self.IsInSpawnCustomisation` false)
        (set `self.IsInRegularCustomisation` true)
        (`/Game/BPs/Utilitys/ErrorAndWarningSignals.PrintDebugLog` "Entering RegularCustomisation!" self)
        (message `/Game/BPs/Interfaces/CustomisationInterface.InitRegularCustomisation` `Object to customise`)))
    (else
      (`/Game/BPs/Utilitys/ErrorAndWarningSignals.PrintError` "Attempted to start customising an invalid object!"))))

(fn `ExitCustomisation`
  (params (ExitType :type "/Game/BPs/Customisation/Enums/SubModeExitType Enum" :default "NewEnumerator0"))
  (bind _selectedactor (`self.SelectedActor`))
  (if (`KismetSystemLibrary.IsValid` (`self.SelectedActor`))
    (if (`self.IsInSpawnCustomisation`)
      (set `self.IsInSpawnCustomisation` false)
      (`/Game/BPs/Utilitys/ErrorAndWarningSignals.PrintDebugLog` "Sending End-Creation-Customisation-Request!" self)
      (message `/Game/BPs/Interfaces/CustomisationInterface.EndPostCreationCustomisation` _selectedactor ExitType)
      (elif (`self.IsInRegularCustomisation`)
        (set `self.IsInRegularCustomisation` false)
        (`/Game/BPs/Utilitys/ErrorAndWarningSignals.PrintDebugLog` "Sending End-Regular-Customisation-Request!" self)
        (message `/Game/BPs/Interfaces/CustomisationInterface.EndRegularCustomisation` _selectedactor ExitType)
        (else
          (`/Game/BPs/Utilitys/ErrorAndWarningSignals.PrintWarning` "Attempted to Exit Customisation, but was neither in Regular nor Spawn Customisation mode."))))
    (else
      (`/Game/BPs/Utilitys/ErrorAndWarningSignals.PrintError` "Attempted to exit customisation of object, but no valid object was selected as focus!"))))

(fn `GetCustomisationStates`
  (returns (SpawnCustomisation :type Boolean) (RegularCustomisation :type Boolean))
  (return (`self.IsInSpawnCustomisation`) (`self.IsInRegularCustomisation`)))

(fn `GetSelectedReferences`
  (returns (Actor :type "Actor Object Reference") (Class :type "Actor Class Reference"))
  (return (`self.SelectedActor`) (`self.SelectedClass`)))

(fn `HasValidActorSelection`
  (returns (HasValidSelection :type Boolean))
  (return (`KismetSystemLibrary.IsValid` (`self.SelectedActor`))))

(fn `HasValidClassSelection`
  (returns (HasValidSelection :type Boolean))
  (return (`KismetSystemLibrary.IsValidClass` (`self.SelectedClass`))))

(fn `IsInSpawnInMode`
  (returns (IsInSpawningMode :type Boolean))
  (return (`KismetSystemLibrary.IsValidClass` (`self.SelectedClass`))))

(fn `MakeNewSelection`
  (params (NewSelection :type "Actor Object Reference"))
  (bind _output_get (set `self.SelectedActor` NewSelection))
  (`/Game/BPs/Utilitys/ErrorAndWarningSignals.PrintDebugLog` "Selected new Object!" self)
  (bind _aseditor_ui (cast `/Game/UMG/EditorUI` (`self.MainEditorUI`)))
  (`/Game/UMG/EditorUI.New Selected Object` _aseditor_ui _output_get)
  (message `/Game/BPs/Interfaces/SelectionInterface.RegisterSelection` _output_get))

(fn `SelectNewObject`
  (params (ActorInstance :type "Actor Object Reference") (ActorClass :type "Actor Class Reference"))
  (bind _returnvalue (`KismetSystemLibrary.IsValid` ActorInstance))
  (bind _returnvalue_2 (`KismetSystemLibrary.IsValidClass` ActorClass))
  ;[1 1 1] Error Checking
  (if (or (and _returnvalue _returnvalue_2) (not (or _returnvalue _returnvalue_2)))
    (`/Game/BPs/Utilitys/ErrorAndWarningSignals.PrintError` "Misuse of SelectNewObject-Function! Only supply an Instance OR a Class, never both and allways one of them! See Tooltip for more info.")
    (else
      ;[1 1 1] Deselect Previous Selection
      (`self.UnSelectCurrentSelection`)
      (if _returnvalue
        (`self.MakeNewSelection` ActorInstance)
        (set `self.SelectedClass` null)
        (else
          (set `self.SelectedClass` ActorClass)
          (set `self.SelectedActor` null)
          (`/Game/BPs/Utilitys/ErrorAndWarningSignals.PrintDebugLog` "New Class selection made!" self))))))

(fn `SpawnNewObject`
  (params (Hit :type "HitResult Structure"))
  (returns (NewObject :type "Actor Object Reference"))
  (bind _returnvalue (`|SpawnActorFromClass` (`self.SelectedClass`) (`KismetMathLibrary.MakeTransform` (`.Location` (`GameplayStatics.BreakHitResult` Hit))) "AlwaysSpawn" "OverrideRootScale" null null))
  (`self.SelectNewObject` _returnvalue)
  (`self.EnterCustomisation` _returnvalue)
  (bind _aseditor_ui (cast `/Game/UMG/EditorUI` (`self.MainEditorUI`)))
  (`/Game/UMG/EditorUI.RefreshSceneList` _aseditor_ui)
  (return _returnvalue))

(fn `UnSelectCurrentSelection`
  (bind _selectedactor (`self.SelectedActor`))
  (`/Game/BPs/Utilitys/ErrorAndWarningSignals.PrintDebugLog` "Unselecting currently selected object if exsisting!" self)
  (if (`KismetSystemLibrary.IsValid` _selectedactor)
    (`/Game/BPs/Utilitys/ErrorAndWarningSignals.PrintDebugLog` "Unregistering Selection and Exiting Customiation." self)
    ;[1 1 1] Clear up selection
    (message `/Game/BPs/Interfaces/SelectionInterface.UnRegisterSelection` _selectedactor)
    ;[1 1 1] Exit Customisation of current selection
    (`self.UpdateSpawnCustomisationState` false)
    (`self.UpdateRegularCustomisationState` false))
  ;[1 1 1] Empty References to Objects
  (set `self.SelectedActor` null)
  (set `self.SelectedClass` null))

(fn `UpdatePerspective`
  (bind _returnvalue (`SceneComponent.K2_GetComponentLocation` (`self.TopDownCamera`)))
  (if (`self.IsFirstPerson`)
    (bind _outhit (`KismetSystemLibrary.LineTraceSingle` _returnvalue (`KismetMathLibrary.MakeVector` (.x _returnvalue) (.y _returnvalue) -10000.0) "TraceTypeQuery1" true))
    (`self.K2_SetActorTransform` (`KismetMathLibrary.MakeTransform` (+ (`.Location` (`GameplayStatics.BreakHitResult` _outhit)) (0.0 0.0 100.0)) (.rotation (stale _output_get))))
    (`ActorComponent.SetActive` (`self.TopDownCamera`) false false)
    (`ActorComponent.SetActive` (`self.FirstPersonCamera`) true false)
    (bind _returnvalue_2 (`GameplayStatics.GetActorOfClass` "/SunPosition/SunSky.SunSky_C"))
    (`LightComponentBase.SetCastShadows` (`/SunPosition/SunSky.DirectionalLight` _returnvalue_2) true)
    (else
      (bind _output_get (set `self.FirstPersonTransform` (`self.GetTransform`)))
      (`ActorComponent.SetActive` (`self.FirstPersonCamera`) false false)
      (`ActorComponent.SetActive` (`self.TopDownCamera`) true false)
      (`self.K2_SetActorTransform` (`KismetMathLibrary.MakeTransform` (`self.K2_GetActorLocation`)))
      (bind _returnvalue_3 (`GameplayStatics.GetActorOfClass` "/SunPosition/SunSky.SunSky_C"))
      (`LightComponentBase.SetCastShadows` (`/SunPosition/SunSky.DirectionalLight` _returnvalue_3) false))))

(fn `UpdateRegularCustomisationState`
  (params (NewRegularCustomisationState :type Boolean))
  (if (not (== NewRegularCustomisationState (`self.IsInRegularCustomisation`)))
    (if NewRegularCustomisationState
      (`self.EnterCustomisation` (`self.SelectedActor`) "NewEnumerator1")
      (else
        (`self.ExitCustomisation` "NewEnumerator0")))))

(fn `UpdateSpawnCustomisationState`
  (params (NewSpawnCustomisationState :type Boolean))
  (if (not (== NewSpawnCustomisationState (`self.IsInSpawnCustomisation`)))
    (if NewSpawnCustomisationState
      (`self.EnterCustomisation` (`self.SelectedActor`))
      (else
        (`self.ExitCustomisation` "NewEnumerator0")))))

(fn `UserConstructionScript`)