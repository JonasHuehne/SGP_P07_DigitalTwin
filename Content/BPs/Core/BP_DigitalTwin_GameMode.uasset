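; Game mode for a digital twin project that holds the shared grid unit size and simulation state, each exposed through getter and setter functions.
; Setting the grid size also writes it to the GridInterval scalar in the PP_ParameterCollection material parameter collection, keeping materials that read it in sync.
; Setting the simulation state stores it and broadcasts the SimulationStateUpdated event dispatcher with the new state.
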(event `self.ReceiveBeginPlay`)

(fn `GetGridSize`
  (returns (GridSize :type "Float (double-precision)"))
  (return (`self.GridUnitSize`)))

(fn `GetSimulationState`
  (returns (SimulationState :type "/Game/BPs/Simulation/SimulationState Enum"))
  (return (`self.SimulationState`)))

(fn `SetGridSize`
  (params (NewGridSize :type "Float (double-precision)"))
  (bind _output_get (set `self.GridUnitSize` NewGridSize))
  (`KismetMaterialLibrary.SetScalarParameterValue` "/Game/Materials/PP/PP_ParameterCollection.PP_ParameterCollection" "GridInterval" _output_get))

(fn `SetSimulationState`
  (params (SimulationState :type "/Game/BPs/Simulation/SimulationState Enum" :default "NewEnumerator0"))
  (bind _output_get (set `self.SimulationState` SimulationState))
  (`self.SimulationStateUpdated` _output_get)
  (return))

(fn `UserConstructionScript`)